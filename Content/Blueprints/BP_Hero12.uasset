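; BP_Hero12 is a 2D Paper flipbook hero character that sets its hand flipbook on BeginPlay.
; Tick copies IsShooting into IsShootingBP each frame, working around the C++ variable misbehaving in the state machine.
; Graphs for timed dashing, direction-based sprite flipping with mouse-angle hand aiming, gun socket attachment and shooting are present but disconnected, and the overlap event is empty.
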(event `EnhancedInput|/Game/Blueprints/Input/Actions/IA_Dash`
  (params (ActionValue :type Boolean) (ElapsedSeconds :type "Float (double-precision)") (TriggeredSeconds :type "Float (double-precision)") (InputAction :type "InputAction Object Reference" :default "/Game/Blueprints/Input/Actions/IA_Dash.IA_Dash"))
  ;[1 0.7865 0.7466] Dash
  ;;[1 1 1] Dash Input Action
)

(event `self.ReceiveBeginPlay`
  (`PaperFlipbookComponent.SetFlipbook` (`self.HandComponent`) "/Game/Assets/Player/FB_Hero_Hand.FB_Hero_Hand") ; idk why HandComponent is broken so I had to do this manuelly
)

(event `self.ReceiveTick`
  (params (DeltaSeconds :type "Float (single-precision)"))
  (set `self.IsShootingBP` (`self.IsShooting`)) ; Idk why Is Shooting C++ variable doesn't work correct in state machine \neven though when I print it prints correct. I used this method and it worked
)

(event `self.BoxComponent.OnComponentBeginOverlap`
  (params (OverlappedComponent :type "PrimitiveComponent Object Reference") (OtherActor :type "Actor Object Reference") (OtherComp :type "PrimitiveComponent Object Reference") (OtherBodyIndex :type Integer) (bFromSweep :type Boolean) (SweepResult :type "HitResult Structure (by ref)"))
  ;[1 1 1] Attaching Gun to HandSocket
)

(event `EnhancedInput|/Game/Blueprints/Input/Actions/IA_Shoot`
  (params (ActionValue :type Boolean) (ElapsedSeconds :type "Float (double-precision)") (TriggeredSeconds :type "Float (double-precision)") (InputAction :type "InputAction Object Reference" :default "/Game/Blueprints/Input/Actions/IA_Shoot.IA_Shoot"))
  ;[1 1 1] Shooting
)

(fn `UserConstructionScript`)