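; BP_GunBase is a gun base Blueprint whose BeginPlay, Tick and Shoot events are all empty.
; Its graph keeps disconnected logic that never runs: caching the player's BP_Hero12 and accumulating a Pressed timer while that hero is shooting.
; Another disconnected chain would reset the timer at a threshold, spawn BP_Projectile_RogueSpecial at the arrow component, set its velocity and rotate it to the hero's mouse angle.
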(event `self.ReceiveBeginPlay`)

(event `self.ReceiveTick`
  (params (DeltaSeconds :type "Float (single-precision)"))
  ;[1 1 1] Increment Timre if RIght Pressed
)

(event `Shoot`
  ;[1 1 1] Shoot
)

(fn `UserConstructionScript`)