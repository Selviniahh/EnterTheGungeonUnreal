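; BP_RogueSpecial is a gun Blueprint, apparently for the Rogue's special weapon, whose firing logic is currently inactive.
; On BeginPlay it stops and hides its muzzle flash, while its Shoot event is empty.
; Disconnected leftover nodes would cache the player's BP_Hero, accumulate time while it shoots, and periodically spawn a projectile from the arrow, rotated to the mouse angle.
; That spawn node has no actor class set.
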(event `Shoot`
  ;[1 1 1] Shoot
)

(event `self.ReceiveBeginPlay`
  (bind _muzzleflash (`self.MuzzleFlash`))
  (`PaperFlipbookComponent.Stop` _muzzleflash)
  (`SceneComponent.SetVisibility` _muzzleflash false false))

(fn `UserConstructionScript`)