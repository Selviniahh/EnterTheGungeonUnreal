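; BP_RubberBullet is an enemy Blueprint that drives hit and death animations from its health state.
; Each tick it polls HealthComponent, jumping the AnimComponent's anim instance to the GotHit node while damaged and, once dead, to Die through a DoOnce.
; BeginPlay sets a MoveRange value, but no movement logic appears in these graphs.
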(event `self.ReceiveBeginPlay`
  (set `self.MoveRange` 200.0))

(event `self.ReceiveTick`
  (params (DeltaSeconds :type "Float (single-precision)"))
  (if (not (`HealthComponent.IsDead` (`self.HealthComponent`)))
    ;[1 1 1] Play hit if got hit
    (if (`HealthComponent.Damaged` (`self.HealthComponent`))
      (`PaperZDAnimInstance.JumpToNode` (`PaperZDAnimationComponent.AnimInstance` (`self.AnimComponent`)) "GotHit" "None"))
    (else
      ;[1 1 1] If it's dead play death
      (`/Engine/EditorBlueprintResources/StandardMacros.DoOnce` false
        (:`Completed`
          (`PaperZDAnimInstance.JumpToNode` (`PaperZDAnimationComponent.AnimInstance` (`self.AnimComponent`)) "Die" "None"))))))

(fn `UserConstructionScript`)