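; Grenade enemy Blueprint that drives animation from state flags and removes the actor after death.
; Each Tick, after the parent Tick and only while not shooting, it jumps the AnimInstance to Explotee, Leap or GotHit, in that priority, while alive.
; When HealthComponent reports death, it plays Die and destroys the actor after a short delay.
; DoOnce gates keep the explode, leap and death jumps from retriggering every frame.
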(event `self.ReceiveTick`
  (params (DeltaSeconds :type "Float (single-precision)"))
  (`parent.ReceiveTick` DeltaSeconds)
  (bind _output_get (set `self.ShootingBP` (`self.IsShooting`)))
  (if _output_get
    _
    (elif (not (`HealthComponent.IsDead` (`self.HealthComponent`)))
      ;[1 1 1] Explode
      (if (`self.Explode`)
        (`/Engine/EditorBlueprintResources/StandardMacros.DoOnce` false
          (:`Completed`
            (`PaperZDAnimInstance.JumpToNode` (`PaperZDAnimationComponent.AnimInstance` (`self.AnimComponent`)) "Explotee" "None")))
        (else
          ;[1 1 1] Leap
          (if (`self.Leap`)
            (`/Engine/EditorBlueprintResources/StandardMacros.DoOnce` false
              (:`Completed`
                (`PaperZDAnimInstance.JumpToNode` (`PaperZDAnimationComponent.AnimInstance` (`self.AnimComponent`)) "Leap" "None")))
            (else
              ;[1 1 1] Play hit if got hit
              (if (`HealthComponent.Damaged` (`self.HealthComponent`))
                (`PaperZDAnimInstance.JumpToNode` (`PaperZDAnimationComponent.AnimInstance` (`self.AnimComponent`)) "GotHit" "None"))))))
      (else
        ;[1 1 1] If it's dead play death
        (`/Engine/EditorBlueprintResources/StandardMacros.DoOnce` false
          (:`Completed`
            (`PaperZDAnimInstance.JumpToNode` (`PaperZDAnimationComponent.AnimInstance` (`self.AnimComponent`)) "Die" "None")
            (`KismetSystemLibrary.Delay` 1.2)
            (`self.K2_DestroyActor`)))))))

(fn `UserConstructionScript`)