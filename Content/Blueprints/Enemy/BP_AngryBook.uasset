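; Angry book enemy Blueprint that handles the character's death sequence.
; Tick copies IsShooting into ShootingBP and checks the health component's dead state only while the book is not shooting.
; On death, a DoOnce jumps the anim instance to its Die node, waits briefly, then zeroes movement velocity and sets IsDead.
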(event `self.ReceiveBeginPlay`)

(event `self.ReceiveTick`
  (params (DeltaSeconds :type "Float (single-precision)"))
  (bind _output_get (set `self.ShootingBP` (`self.IsShooting`)))
  (if _output_get
    _
    (elif (`HealthComponent.IsDead` (`self.HealthComponent`))
      ;[1 1 1] If it's dead play death
      (`/Engine/EditorBlueprintResources/StandardMacros.DoOnce` false
        (:`Completed`
          (`PaperZDAnimInstance.JumpToNode` (`PaperZDAnimationComponent.AnimInstance` (`self.AnimComponent`)) "Die" "None")
          (`KismetSystemLibrary.Delay` 0.5)
          (set `MovementComponent.Velocity` (0.0 0.0 0.0) (`self.MovementComponent`))
          (set `self.bIsDead` true))))))

(fn `UserConstructionScript`)