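; Shotgun Bullet Man enemy Blueprint that adds death handling on top of its parent class.
; Each Tick runs the parent logic, then copies IsShooting into ShootingBP.
; When it is not shooting and its HealthComponent reports dead, a DoOnce jumps the animation instance to the "Die" node.
; The actor then destroys itself after a short delay.
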(event `self.ReceiveTick`
  (params (DeltaSeconds :type "Float (single-precision)"))
  (`parent.ReceiveTick` DeltaSeconds)
  (bind _output_get (set `self.ShootingBP` (`self.IsShooting`)))
  (if _output_get
    _
    (elif (not (not (`HealthComponent.IsDead` (`self.HealthComponent`))))
      ;[1 1 1] If it's dead play death
      (`/Engine/EditorBlueprintResources/StandardMacros.DoOnce` false
        (:`Completed`
          (`PaperZDAnimInstance.JumpToNode` (`PaperZDAnimationComponent.AnimInstance` (`self.AnimComponent`)) "Die" "None")
          (if (`HealthComponent.IsDead` (`self.HealthComponent`))
            (`KismetSystemLibrary.Delay` 0.5)
            (`self.K2_DestroyActor`)))))))

(fn `UserConstructionScript`)