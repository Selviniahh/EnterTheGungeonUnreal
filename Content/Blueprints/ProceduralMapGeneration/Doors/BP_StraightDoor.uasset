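; BP_StraightDoor is a double door for procedural map generation that opens when the hero walks into its trigger box.
; Its two flipbook halves, DoorFBRight and DoorFBLeft, start paused and non-looping on BeginPlay, though only the left one has its time reset.
; A BP_Hero overlap with the box sets both play rates to normal, and no logic closes the door again.
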(event `self.ReceiveBeginPlay`
  (bind _doorfbright (`self.DoorFBRight`))
  (bind _doorfbleft (`self.DoorFBLeft`))
  (`PaperFlipbookComponent.SetPlayRate` _doorfbright 0.0)
  (`PaperFlipbookComponent.SetPlayRate` _doorfbleft 0.0)
  (`PaperFlipbookComponent.SetLooping` _doorfbright false)
  (`PaperFlipbookComponent.SetLooping` _doorfbleft false)
  (`PaperFlipbookComponent.SetNewTime` _doorfbleft 0.0)
  (`PaperFlipbookComponent.SetNewTime` _doorfbleft 0.0))

(event `self.BoxComponent.OnComponentBeginOverlap`
  (params (OverlappedComponent :type "PrimitiveComponent Object Reference") (OtherActor :type "Actor Object Reference") (OtherComp :type "PrimitiveComponent Object Reference") (OtherBodyIndex :type Integer) (bFromSweep :type Boolean) (SweepResult :type "HitResult Structure (by ref)"))
  (cast `/Game/Blueprints/BP_Hero` OtherActor)
  (`PaperFlipbookComponent.SetPlayRate` (`self.DoorFBRight`) 1.0)
  (`PaperFlipbookComponent.SetPlayRate` (`self.DoorFBLeft`) 1.0))

(fn `UserConstructionScript`)