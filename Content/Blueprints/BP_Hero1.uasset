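; BP_Hero1 is a 2D flipbook hero that faces its current direction and picks up a gun on contact.
; Tick pins the FlipBook to a fixed world height and mirrors it by negative scale unless CurrentDirection is one of the right-side values.
; When its BoxComponent overlaps a BP_Gun_RogueSpecial, it stores the gun's flipbook as GunSprite and attaches the gun to the Asd component, snapping location and keeping relative rotation and scale.
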(event `self.ReceiveTick`
  (params (DeltaSeconds :type "Float (single-precision)"))
  (bind _flipbook (`self.FlipBook`))
  (bind _currentdirection (`self.CurrentDirection`))
  (bind (_returnvalue_x _returnvalue_y) (`KismetMathLibrary.BreakVector` (`SceneComponent.K2_GetComponentLocation` _flipbook)))
  (`SceneComponent.K2_SetWorldLocation` _flipbook (`KismetMathLibrary.MakeVector` _returnvalue_x _returnvalue_y -246.0) false false)
  (if (or (`|EnumEquality` _currentdirection "Right") (`|EnumEquality` _currentdirection "Front_Hand_Right") (`|EnumEquality` _currentdirection "Back_Diagonal_Right") (`|EnumEquality` _currentdirection "Back_Hand_Right"))
    (`SceneComponent.SetRelativeScale3D` (`self.FlipBook`) (1.0 1.0 1.0)) ; don't flip
    (else
      (`SceneComponent.SetRelativeScale3D` (`self.FlipBook`) (-1.0 -1.0 1.0)) ; Flip sprite
    )))

(event `self.BoxComponent.OnComponentBeginOverlap`
  (params (OverlappedComponent :type "PrimitiveComponent Object Reference") (OtherActor :type "Actor Object Reference") (OtherComp :type "PrimitiveComponent Object Reference") (OtherBodyIndex :type Integer) (bFromSweep :type Boolean) (SweepResult :type "HitResult Structure (by ref)"))
  (bind _asbp_gun_rogue_special (cast `/Game/Blueprints/Guns/BP_Gun_RogueSpecial` OtherActor))
  (set `self.Gun Sprite` (`/Game/Blueprints/Guns/BP_Gun_Parent.PaperFlipbook` _asbp_gun_rogue_special))
  (`self.K2_AttachToComponent` _asbp_gun_rogue_special (`self.asd`) "None" "SnapToTarget" "KeepRelative" "KeepRelative" true))

(fn `UserConstructionScript`)